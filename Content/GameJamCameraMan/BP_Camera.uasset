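; BP_Camera is a camera actor that tracks the player's VR pawn and blinks a red light.
; On BeginPlay, a looping one-second timer toggles the RedLight's visibility.
; Every Tick, it casts the player pawn to VRPawn and rotates ROTATIONBALL2 to look at that pawn's camera.
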(event Custom|ClignotingLight
  (bind _redlight (Variables|Default|GetRedLight))
  (if (Rendering|IsVisible _redlight)
    (Rendering|SetVisibility _redlight false false)
    (else
      (Rendering|SetVisibility _redlight true false))))

(event EventBeginPlay
  (Utilities|Time|SetTimerbyEvent (delegate Custom|ClignotingLight) 1.0 true))

(event EventTick
  (params (DeltaSeconds :type Float%20%28single-precision%29))
  (bind _asvrpawn (Utilities|Casting|CastToVRPawn (Game|Player|GetPlayerPawn 0)))
  (Transformation|SetWorldRotation (Variables|Default|GetROTATIONBALL2) (Math|Rotator|FindLookatRotation (Transformation|GetWorldLocation (Variables|Default|GetROTATIONBALL2)) (Transformation|GetWorldLocation (Variables|/Game/VRTemplate/Blueprints/VRPawn.VRPawn_C|GetCamera _asvrpawn))) false false))

(fn ConstructionScript)