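; PC_BP is a computer for a VR switch puzzle, with a screen and point light showing its on or off state.
; Switch toggles it and every PC in its linked array, then asks VRPawn to check whether all are on.
; SwitchOnOff derives the current state from the light color, swapping screen material and red or blue light.
; AllScreensOnClignoting plays a delayed blink that leaves the screen lit green.
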(event Custom|AllScreensOnClignoting
  (bind _screen (Variables|Default|GetScreen))
  (bind _pointlight (Variables|Default|GetPointLight))
  (Utilities|FlowControl|Delay 1.0)
  (Rendering|Material|SetMaterial _screen 0 "/Game/GameJamCameraMan/Materials/ScreenOff_M.ScreenOff_M")
  (Rendering|Components|Light|SetIntensity _pointlight 0.0)
  (Utilities|FlowControl|Delay 0.35)
  (Rendering|Material|SetMaterial _screen 0 "/Game/GameJamCameraMan/Materials/ScreenOn_M.ScreenOn_M")
  (Rendering|Components|Light|SetIntensity _pointlight 2.0)
  (Rendering|Components|Light|SetLightColor _pointlight "(R=0.003097,G=1.000000,B=0.000000,A=1.000000)" true)
  (Utilities|FlowControl|Delay 0.35)
  (Rendering|Material|SetMaterial _screen 0 "/Game/GameJamCameraMan/Materials/ScreenOff_M.ScreenOff_M")
  (Rendering|Components|Light|SetIntensity _pointlight 0.0)
  (Utilities|FlowControl|Delay 0.35)
  ;[1 1 1] mettre image
  (Rendering|Material|SetMaterial _screen 0 "/Game/GameJamCameraMan/Materials/ScreenOn_M.ScreenOn_M")
  (Rendering|Components|Light|SetIntensity _pointlight 2.0))

(event EventSwitch
  (CallFunction|SwitchonOff)
  (for _array_element (Variables|Default|GetPC_InstancesArray)
    (CallFunction|SwitchonOff _array_element))
  (bind _asvrpawn (Utilities|Casting|CastToVRPawn (Game|Player|GetPlayerPawn 0)))
  (Default|CallCheckAllPCon _asvrpawn))

(fn ConstructionScript)

(fn SwitchonOff
  (bind _screen (Variables|Default|GetScreen))
  (bind _pointlight (Variables|Default|GetPointLight))
  (if (Class|KismetMathLibrary|LinearColorIsNearEqual (Rendering|Components|Light|GetLightColor (Variables|Default|GetPointLight)) "(R=1.000000,G=0.000000,B=0.014444,A=1.000000)" 0.0001)
    (Rendering|Material|SetMaterial _screen 0 "/Game/GameJamCameraMan/Materials/ScreenOn_M.ScreenOn_M")
    (Rendering|Components|Light|SetLightColor _pointlight "(R=0.000000,G=0.077525,B=0.677083,A=1.000000)" true)
    (Variables|Default|SetIsScreenTurnedOn true)
    (else
      (Rendering|Material|SetMaterial _screen 0 "/Game/GameJamCameraMan/Materials/ScreenOff_M.ScreenOff_M")
      (Rendering|Components|Light|SetLightColor _pointlight "(R=1.000000,G=0.000000,B=0.014444,A=1.000000)" true)
      (Variables|Default|SetIsScreenTurnedOn false))))